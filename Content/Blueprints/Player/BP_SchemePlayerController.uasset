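; Player controller for a turn-based networked game, handling mouse look and player requests to the server.
; On BeginPlay, the local controller adds the Scheme Enhanced Input mapping context, and mouse look input feeds a clamped rotation handler.
; Hard-bound debug-style keys send server requests: E to finish the turn, with an on-screen print, and F to start the game.
; The rotation and request functions are called here but defined outside these graphs.
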(event Input|EnhancedActionEvents|EnhancedInputActionIA_MouseLook
  (params (ActionValue :type Vector%202D%20Structure) (ElapsedSeconds :type Float%20%28double-precision%29) (TriggeredSeconds :type Float%20%28double-precision%29) (InputAction :type Input%20Action%20Object%20Reference :default "/Game/InputSystem/IA_MouseLook.IA_MouseLook"))
  (Class|SchemePlayerController|HandleClampedRotation (.x ActionValue) (.y ActionValue)))

(event EventBeginPlay
  (if (Pawn|IsLocalPlayerController)
    (Input|AddMappingContext (PlayerController|LocalPlayerSubsystems|GetEnhancedInputLocalPlayerSubsystem) "/Game/InputSystem/IM_SchemeInputMapping.IM_SchemeInputMapping" 0 "(bIgnoreAllPressedKeysUntilRelease=True,bForceImmediately=False,bNotifyUserSettings=False)")))

(event EventTick
  (params (DeltaSeconds :type Float%20%28single-precision%29)))

(event Input|KeyboardEvents|E
  (params (Key :type Key%20Structure :default "None"))
  (:Pressed
    (Development|PrintString "Sending Request" true false)
    (Class|SchemePlayerController|SendServerFinishTurnRequest)))

(event Input|KeyboardEvents|F
  (params (Key :type Key%20Structure :default "None"))
  (:Pressed
    (Class|SchemePlayerController|SendGameStartRequesttoServer)))

(fn ConstructionScript)