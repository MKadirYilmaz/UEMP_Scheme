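; BP_SchemePlayerPawn is a player pawn that can interact and be interacted with through an action UI.
; The primary input action asks InteractionComp to attempt an interaction.
; On client-side interaction success, it creates WB_ActionInterface for the interactor's controller, fills it with gold from this pawn's own PlayerState, and shows the cursor.
; The construction script sets Root to absolute location, rotation and scale.
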(event Input|EnhancedActionEvents|EnhancedInputActionIA_PrimaryAction
  (params (ActionValue :type Boolean) (ElapsedSeconds :type Float%20%28double-precision%29) (TriggeredSeconds :type Float%20%28double-precision%29) (InputAction :type Input%20Action%20Object%20Reference :default "/Game/InputSystem/IA_PrimaryAction.IA_PrimaryAction"))
  (Class|InteractionComponent|TryPrimaryInteract (Variables|Default|GetInteractionComp)))

(event EventOnInteract
  (params (Interactor :type Pawn%20Object%20Reference)))

(event Collision|EventActorBeginOverlap
  (params (OtherActor :type Actor%20Object%20Reference)))

(event EventTick
  (params (DeltaSeconds :type Float%20%28single-precision%29)))

(event EventOnInteractionSuccessinClient
  (params (Interactor :type Pawn%20Object%20Reference))
  (Development|PrintString (Utilities|GetDisplayName self))
  (bind _asbp_scheme_player_controller (Utilities|Casting|CastToBP_SchemePlayerController (Pawn|GetController Interactor)))
  (Utilities|FlowControl|Sequence
    (:then_0
      (bind _returnvalue (UserInterface|CreateWidget "/Game/Blueprints/UIWidget/WB_ActionInterface.WB_ActionInterface_C" _asbp_scheme_player_controller)))
    (:then_1
      (bind _asbp_scheme_player_state (Utilities|Casting|CastToBP_SchemePlayerState (Variables|Default|GetPlayerState)))
      (Default|SetPlayerGold _returnvalue (Class|SchemePlayerState|GetGold _asbp_scheme_player_state)))
    (:then_2
      (UserInterface|Viewport|AddtoViewport _returnvalue 0)
      (Variables|/Script/Engine.PlayerController|SetbShowMouseCursor _asbp_scheme_player_controller true))))

(fn ConstructionScript
  (Transformation|SetAbsolute (Variables|Default|GetRoot) true true true))