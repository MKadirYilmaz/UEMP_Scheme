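; BP_GoldPile is an interactable gold pile actor that requests gold income for the player and shows a gold pile UI.
; On interact, a locally controlled interactor's BP_SchemePlayerController sends the server a gold income request, marked as a gold system test.
; Client-side interaction success creates the gold pile widget and disables camera rotation, behind a DoOnce with no reset here.
; The focus events are empty stubs.
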(event EventBeginPlay)

(event Collision|EventActorBeginOverlap
  (params (OtherActor :type Actor%20Object%20Reference)))

(event EventTick
  (params (DeltaSeconds :type Float%20%28single-precision%29)))

(event EventOnInteract
  (params (Interactor :type Pawn%20Object%20Reference))
  (if (Pawn|IsLocallyControlled Interactor)
    ;[0.15 0.15 0.15 0.5] Test Gold System
    (bind _asbp_scheme_player_controller (Utilities|Casting|CastToBP_SchemePlayerController (Pawn|GetController Interactor)))
    (Class|SchemePlayerController|SendGoldIncomeRequesttoServer _asbp_scheme_player_controller 2)))

(event EventOnBeginFocus
  (params (Interactor :type Pawn%20Object%20Reference))
  (if (Pawn|IsLocallyControlled Interactor)
    _))

(event EventOnEndFocus
  (params (Interactor :type Pawn%20Object%20Reference))
  (if (Pawn|IsLocallyControlled Interactor)
    _))

(event EventOnInteractionSuccessinClient
  (params (Interactor :type Pawn%20Object%20Reference))
  (bind _asplayer_controller (Utilities|Casting|CastToPlayerController (Pawn|GetController Interactor)))
  (Utilities|FlowControl|DoOnce false
    (:Completed
      (bind _returnvalue (UserInterface|CreateWidget "/Game/Static/UI/SlotsOf3/GoldPileWidget.GoldPileWidget_C" _asplayer_controller))
      (UserInterface|Viewport|AddtoViewport _returnvalue 0)
      (bind _asbp_scheme_player_controller (Utilities|Casting|CastToBP_SchemePlayerController _asplayer_controller))
      (Class|SchemePlayerController|SetCameraRotationEnabled _asbp_scheme_player_controller false))))

(fn ConstructionScript)